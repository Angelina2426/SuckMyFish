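; Base fish character that swims by physics and movement input, flees the player and reacts to being vacuumed.
; FindSwimResult builds steering from random targets, three obstacle traces and player avoidance, feeding swim, flee and Tolkyn movement events.
; Tick applies flag-driven flee, vacuum struggle and damped "blackhole" pull toward the capsule.
; It also handles coral cleaning, speed boosts and material variants; BeginPlay is empty, with swim-timer setup disconnected.
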(event `self.ReceiveBeginPlay`)

(event `swimEvent`
  (bind _returnvalue (`KismetMathLibrary.RandomFloatInRange` 0.1 0.45))
  (bind _scale_value (`self.Scale Value`))
  (bind _scale_value_2 (`self.Scale Value`))
  ;[0.15 0.007041 0.09538 0.5] тот самый ивент пж не трогай тут ничего иначе рыбой стану я (оно работает на добром слове анрила анрилыча)
  (`self.FindSwimResult`)
  (`self.find tricky run vector`)
  (`self.AddMovementInput` (`self.velocity`) _scale_value)
  (`self.FindSwimResult`)
  (`KismetSystemLibrary.Delay` _returnvalue)
  (`self.AddMovementInput` (`self.velocity`) _scale_value)
  (`self.FindSwimResult`)
  (`KismetSystemLibrary.Delay` _returnvalue)
  (`self.AddMovementInput` (`self.velocity`) _scale_value_2)
  (`self.FindSwimResult`)
  (`KismetSystemLibrary.Delay` (`KismetMathLibrary.RandomFloatInRange` 0.1 0.45))
  (`self.AddMovementInput` (`self.velocity`) _scale_value_2))

(event `speedup`
  ;[0.067 0.15 0.04479 0.5] ускорение рыбы
  (set `self.speedupByTolkyn` 4.5)
  (`KismetSystemLibrary.PrintString` "now i fastr" true true (struct :`R` 0.093001 :`G` 1.0 :`A` 1.0))
  (`KismetSystemLibrary.RetriggerableDelay` 6.0)
  (`KismetSystemLibrary.PrintString` "nope" true true (struct :`R` 1.0 :`B` 0.004913 :`A` 1.0))
  (set `self.speedupByTolkyn` 1.0))

(event `Iwilldie`
  ;[0.15 0 0.08059 0.5] рыба подумает что она умрет...
  (`self.FindSwimResult`)
  (`PrimitiveComponent.SetAllPhysicsLinearVelocity` (`self.er`) (* (* (+ (* (+ (* (`self.trickyrunvector`) 2.0) (`KismetMathLibrary.Normal` (`self.VectorSwim`))) 0.7) (* (`KismetMathLibrary.RandomUnitVector`) 0.3)) (`self.GetActorRightVector`) (`self.Fish Behavior`)) 0.2) true))

(event `self.ReceiveTick`
  (params (DeltaSeconds :type "Float (single-precision)"))
  ;[0.15 0 0.04668 0.5] обосрется рыба или нет (флаги определяются в оружии и персонаже)
  (if (or (not (`self.ezhik`)) (not (`self.iftoklyn`)))
    (`|ExecutionSequence`
      (:`then_0`
        (if (`self.isplayerhere`)
          (`self.INEEDRUN`))
        (if (`self.vaccumbro`)
          (`self.Iwilldie`)))
      (:`then_1`
        (if (`self.blh`)
          (`self.craft`))))))

(event `ivacuumed`
  ;[0.15 0.000618 0.09906 0.5] флаг на поведение рыбы в ивенттике
  (set `self.vaccumbro` true)
  (`KismetSystemLibrary.RetriggerableDelay` 0.2)
  (set `self.vaccumbro` false))

(event `self.ReceiveActorBeginOverlap`
  (params (OtherActor :type "Actor Object Reference"))
  ;[0.3366 0.9271 0 0.5] тут нужна будет обратка -- фул механ полировки ноды
  (if (not (`self.ezhik`))
    (cast `/Game/weaponsystem/WholeVacuumedStuff/BP_Coral_Child` OtherActor)
    (set `self.cleanes_bar` (- (`self.cleanes_bar`) 1))
    (`KismetSystemLibrary.Delay` 0.7)
    (if (and (and (== (`self.cleanes_bar`) 0) (!= (`self.clearness`) true)) (!= (`self.coral`) true))
      (`KismetSystemLibrary.PrintString` "im clear)" true true (struct :`R` 1.0 :`B` 0.095164 :`A` 1.0))
      (set `self.clearness` true)
      (`PrimitiveComponent.SetMaterial` (`self.er`) 0 "/Engine/EngineMeshes/BackgroundMaterial.BackgroundMaterial"))))

(event `INEEDRUN`
  (bind (_velocitytomove_x _velocitytomove_y _velocitytomove_z) (`KismetMathLibrary.BreakVector` (`self.VelocityTomove`)))
  ;[0.15 0 0.09724 0.5] рыба при попадении в колизию игрока начинает жестко валить (смотреть без смс и регистрации в МАКС)
  (`self.FindSwimResult`)
  (`PrimitiveComponent.SetAllPhysicsLinearVelocity` (`self.er`) (`KismetMathLibrary.MakeVector` (* _velocitytomove_x -0.35) (* _velocitytomove_y 0.35) (* _velocitytomove_z 0.35)) true))

(event `Tolkyn_Movement`
  ; толкун мувмент
  (`self.FindSwimResult`)
  (`self.find tricky run vector`)
  (`PrimitiveComponent.SetAllPhysicsLinearVelocity` (`self.er`) (* (`self.VelocityTomove`) (`self.multiplyTolkyn`)) true)
  (`self.FindSwimResult`)
  (`KismetSystemLibrary.Delay` (`KismetMathLibrary.RandomFloatInRange` 0.3 0.7))
  (`PrimitiveComponent.SetAllPhysicsLinearVelocity` (`self.er`) (* (`self.VelocityTomove`) (`self.multiplyTolkyn`)) true)
  (`self.FindSwimResult`))

(event `Tolkyn_Timer`
  ; таймер толкун
  (bind _returnvalue (`KismetSystemLibrary.K2_SetTimerDelegate` (delegate `Tolkyn_Movement`) (`KismetMathLibrary.RandomFloatInRange` 2.0 3.0) true))
  (set `self.swim` _returnvalue))

(fn `angry`
  (`KismetSystemLibrary.PrintString` "IM ANGRY" true true (struct :`G` 1.0 :`B` 0.189135 :`A` 1.0))
  (`PrimitiveComponent.SetMaterial` (`self.er`) 0 "/Game/weaponsystem/WholeVacuumedStuff/materials/M_angryezhik.M_angryezhik"))

(fn `blackhole`
  (returns (blhole :type "Vector Structure"))
  (bind _er (`self.er`))
  (`PrimitiveComponent.SetAngularDamping` _er 100.0)
  (`PrimitiveComponent.SetLinearDamping` _er 70.0)
  (return (* (`KismetMathLibrary.Normal` (- (`SceneComponent.K2_GetComponentLocation` (`self.CapsuleComponent`)) (`SceneComponent.K2_GetComponentLocation` (`self.er`)))) 1500.0)))

(fn `craft`
  (`PrimitiveComponent.SetAllPhysicsLinearVelocity` (`self.er`) (`self.blackhole`) true))

(fn `desicion`
  (set `self.VelocityTomove` (+ (* (+ (- (`self.VectorSwim`) (`SceneComponent.K2_GetComponentLocation` (`self.er`))) (* (`KismetMathLibrary.RandomUnitVector`) (`self.noise`))) 0.95) (`self.Centrer`))))

(fn `find tricky run vector`
  (set `self.trickyrunvector` (+ (`KismetMathLibrary.Cross_VectorVector` (`KismetMathLibrary.Normal` (- (`SceneComponent.K2_GetComponentLocation` (`self.er`)) (`self.K2_GetActorLocation` (`self.playerpawn`)))) (0.0 0.0 1.0)) (* (`self.normalimpact`) 0.6))))

(fn `FindSwimResult`
  (`self.Linetrace(sight1)`)
  (`self.FishFindVector`)
  (`self.desicion`)
  (`self.ifblock(sight2)`)
  (`self.fish prediction`))

(fn `fish prediction`
  (if (`self.isplayerhere`)
    (bind _output_get (set `self.Run` (`KismetMathLibrary.Normal` (- (`SceneComponent.K2_GetComponentLocation` (`self.er`)) (`self.K2_GetActorLocation` (`self.playerpawn`))))))
    (set `self.VelocityTomove` (+ (* _output_get 10.0) (`self.VelocityTomove`)))
    (else
      (set `self.VectorSwim` (+ (* (`self.Home`) (`KismetMathLibrary.RandomFloatInRange` 0.1 0.3)) (`self.VectorSwim`))))))

(fn `FishFindVector`
  (bind _multiply (`self.multiply`))
  (bind _multiply_2 (`self.multiply`))
  (bind _multiply_3 (`self.multiply`))
  (bind (_returnvalue_x _returnvalue_y _returnvalue_z) (`KismetMathLibrary.BreakVector` (`SceneComponent.K2_GetComponentLocation` (`self.er`))))
  (bind _returnvalue (`PrimitiveComponent.GetPhysicsLinearVelocity` (`self.er`) "None"))
  (set `self.vel2` _returnvalue)
  (set `self.noisePercent` (`KismetMathLibrary.RandomFloatInRange` 0.8 1.0))
  (set `self.VectorSwim` (+ (* (`self.vel2`) (+ 1.0 (* (`self.noisePercent`) -1.0))) (`KismetMathLibrary.MakeVector` (* (+ (`KismetMathLibrary.RandomFloatInRange` (* (`self.Min`) _multiply) (* (`self.Max`) _multiply)) _returnvalue_x) (`self.noisePercent`)) (* (+ (`KismetMathLibrary.RandomFloatInRange` (* (`self.Min`) _multiply_3) (* (`self.Max`) _multiply_3)) _returnvalue_y) (`self.noisePercent`)) (* (+ (`KismetMathLibrary.RandomFloatInRange` (* (`self.MinZ`) _multiply_2) (* (`self.MaxZ`) _multiply_2)) _returnvalue_z) (`self.noisePercent`))))))

(fn `ifblock(sight2)`
  (if (or (or (`self.hit3`) (`self.hit`)) (`self.hit2`))
    (set `self.VectorSwim` (* (`self.VectorSwim`) -1.8))))

(fn `Linetrace(sight1)`
  (bind _er (`self.er`))
  (bind _returnvalue (`SceneComponent.K2_GetComponentLocation` _er))
  (bind _returnvalue_2 (`PrimitiveComponent.GetPhysicsLinearVelocity` _er "None"))
  (bind _returnvalue_3 (+ (* (`KismetMathLibrary.Normal` _returnvalue_2) 800.0) _returnvalue))
  (bind (_outhit _returnvalue_4) (`KismetSystemLibrary.LineTraceSingle` _returnvalue (+ _returnvalue_3 (-200.0 0.0 0.0)) "TraceTypeQuery1"))
  (set `self.hit` _returnvalue_4)
  (bind (_outhit_2 _returnvalue_5) (`KismetSystemLibrary.LineTraceSingle` (+ _returnvalue (0.0 0.0 400.0)) (+ _returnvalue (0.0 0.0 -400.0)) "TraceTypeQuery1"))
  (set `self.hit2` _returnvalue_5)
  (bind (_outhit_3 _returnvalue_6) (`KismetSystemLibrary.LineTraceSingle` _returnvalue (+ _returnvalue_3 (500.0 0.0 0.0)) "TraceTypeQuery1"))
  (set `self.hit3` _returnvalue_6)
  (set `self.cornerslop` false)
  (set `self.ImpactNormal` (+ (`.Normal` (`GameplayStatics.BreakHitResult` _outhit_3)) (+ (`.Normal` (`GameplayStatics.BreakHitResult` _outhit_2)) (`.Normal` (`GameplayStatics.BreakHitResult` _outhit))))))

(fn `Linetrace(Tolkyn)`
  (bind _returnvalue (`SceneComponent.K2_GetComponentLocation` (`self.er`)))
  (bind _outhits (`KismetSystemLibrary.SphereTraceMulti` :`Start` _returnvalue :`End` _returnvalue :`Radius` 1000.0 :`TraceChannel` "TraceTypeQuery1" :`DrawDebugType` "ForOneFrame"))
  (for _array_element _outhits
    (bind _asbp_fish_base_character (cast `/Game/weaponsystem/WholeVacuumedStuff/BP_FishBaseCharacter` (`.HitActor` (`GameplayStatics.BreakHitResult` _array_element))))
    (`self.speedup` _asbp_fish_base_character)
    (return)))

(fn `notangry`
  (`KismetSystemLibrary.PrintString` "chiiilll" true true (struct :`G` 1.0 :`B` 0.189135 :`A` 1.0))
  (`PrimitiveComponent.SetMaterial` (`self.er`) 0 "/Game/weaponsystem/WholeVacuumedStuff/materials/M_notangryezh.M_notangryezh"))

(fn `rotationvec`
  (`SceneComponent.K2_SetWorldRotation` (`self.er`) (`KismetMathLibrary.Conv_VectorToRotator` (`KismetMathLibrary.Normal` (`KismetMathLibrary.VInterpTo` (`SceneComponent.K2_GetComponentLocation` (`self.er`)) (`self.VectorSwim`) (`KismetSystemLibrary.GetGameTimeInSeconds`) 15.0))) false false))

(fn `set material`
  (if (`self.ezhik`)
    (`PrimitiveComponent.SetMaterial` (`self.er`) 0 "/Game/weaponsystem/WholeVacuumedStuff/materials/M_notangryezh.M_notangryezh")
    (elif (`|EnumEquality` (`self.fish tag`) "NewEnumerator0")
      (`PrimitiveComponent.SetMaterial` (`self.er`) 0 "/Engine/MapTemplates/Materials/BasicAsset03.BasicAsset03")
      (elif (`|EnumEquality` (`self.fish tag`) "NewEnumerator2")
        (`PrimitiveComponent.SetMaterial` (`self.er`) 0 "/Engine/MapTemplates/Materials/BasicTemplateMaterial.BasicTemplateMaterial")
        (elif (`|EnumEquality` (`self.fish tag`) "NewEnumerator1")
          (`PrimitiveComponent.SetMaterial` (`self.er`) 0 "/Engine/EngineDebugMaterials/BoneWeightMaterial.BoneWeightMaterial"))))))

(fn `stopcraft`
  (params (fish :type Boolean))
  (bind _er (`self.er`))
  (if fish
    (`PrimitiveComponent.SetAngularDamping` _er 4.0)
    (`PrimitiveComponent.SetLinearDamping` _er 1.0)
    (return)))

(fn `StrenthFish`
  (set `self.multiply` (`KismetMathLibrary.RandomFloatInRange` 3.5 5.5)))

(fn `UserConstructionScript`)

(fn `velocity`
  (returns (speed :type "Vector Structure"))
  (return (* (* (`self.VelocityTomove`) (`self.speedupByTolkyn`)) 1000000.0)))