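; Vacuum weapon that pulls BP_FishBase fish toward its muzzle and destroys overlapping fish while Click is set.
; A looping timer runs camera-directed multi-sphere traces, spending ammo and adding velocity to hit fish, with random noise at range.
; Fire and IsClean flip a sign in the pull vector; empty ammo triggers a delayed reload.
; Presets and Sniper/Auto upgrades retune stats, penalizing some mixed branches; SpawnFish launches fish as projectiles.
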(event `self.ReceiveBeginPlay`
  (bind _asbp_third_person_character (cast `/Game/ThirdPerson/Blueprints/BP_ThirdPersonCharacter` (`GameplayStatics.GetPlayerCharacter` 0)))
  (set `self.Follow Camera` (`/Game/ThirdPerson/Blueprints/BP_ThirdPersonCharacter.FollowCamera` _asbp_third_person_character))
  (set `self.As BP Third Person Character` _asbp_third_person_character))

(event `self.ReceiveActorBeginOverlap`
  (params (OtherActor :type "Actor Object Reference"))
  (if (`self.click`)
    (bind _asbp_fish_base (cast `/Game/weaponsystem/WholeVacuumedStuff/BP_FishBase` OtherActor))
    (`self.K2_DestroyActor` _asbp_fish_base)))

(event `end clean`
  (`KismetSystemLibrary.K2_ClearAndInvalidateTimerHandle` (`self.vacuumtimerhandle`)))

(event `startclean`
  (bind _returnvalue (`KismetSystemLibrary.K2_SetTimerDelegate` (delegate `clean`) 0.05 true))
  (set `self.vacuumtimerhandle` _returnvalue))

(event `clean`
  (bind _returnvalue (`SceneComponent.K2_GetComponentLocation` (`self.Scene`)))
  (bind _returnvalue_2 (`KismetMathLibrary.Normal` (`self.distance`)))
  (if (> (`self.current_arm`) 0.0)
    (`self.find_offset`)
    (`KismetSystemLibrary.Delay` (`self.Changable_DelayDuration`))
    (set `self.vacuumsocket` _returnvalue)
    (bind _outhits (`KismetSystemLibrary.SphereTraceMulti` :`Start` (+ _returnvalue (`self.offset`)) :`End` (+ (+ _returnvalue (* (`SceneComponent.GetForwardVector` (`self.Follow Camera`)) (`self.Changeable_VacumDistance`))) (`self.offset`)) :`Radius` (`self.Changeable_Radius`) :`TraceChannel` "TraceTypeQuery1" :`DrawDebugType` "ForDuration"))
    (`self.change arm`)
    (for _array_element _outhits
      (bind _asbp_fish_base (cast `/Game/weaponsystem/WholeVacuumedStuff/BP_FishBase` (`.HitActor` (`GameplayStatics.BreakHitResult` _array_element))))
      (set `/Game/weaponsystem/WholeVacuumedStuff/BP_FishBase.normalimpact` (`.ImpactNormal` (`GameplayStatics.BreakHitResult` _array_element)) _asbp_fish_base)
      (`/Game/weaponsystem/WholeVacuumedStuff/BP_FishBase.stopcraft` _asbp_fish_base (`/Game/weaponsystem/WholeVacuumedStuff/BP_FishBase.blh` _asbp_fish_base))
      (set `/Game/weaponsystem/WholeVacuumedStuff/BP_FishBase.blh` false _asbp_fish_base)
      (`/Game/weaponsystem/WholeVacuumedStuff/BP_FishBase.ivacuumed` _asbp_fish_base)
      (set `self.fishbase` (`/Game/weaponsystem/WholeVacuumedStuff/BP_FishBase.er` _asbp_fish_base))
      ; BasedMovement
      (for _ (range (`self.First Index`) (+ (`self.Last Index`) 1))
        (`self.find_distance`)
        (if (< (`KismetMathLibrary.VSize` (`self.distance`)) 350.0)
          (`PrimitiveComponent.SetAllPhysicsLinearVelocity` (`self.fishbase`) (* _returnvalue_2 (`self.Changeable_vac_forceHigh`)) true)
          (else
            (`PrimitiveComponent.SetAllPhysicsLinearVelocity` (`self.fishbase`) (* (+ _returnvalue_2 (* (`KismetMathLibrary.RandomUnitVector`) (`self.Changeable_noiseVacuum`))) (`self.Changeable_vac_force`)) true)))))
    (else
      (`self.reload`))))

(event `change`
  (`|ExecutionSequence`
    (:`then_0`
      (if (`self.sniperV`)
        (set `self.Changeable_Radius` 25.0)
        (set `self.Changeable_VacumDistance` 1100.0)
        (set `self.Changeable_vac_force` 150.0)
        (set `self.Changeable_speedup` 300.0)
        (set `self.Changeable_vac_forceHigh` 200.0)
        (set `self.Changeable_noiseVacuum` 1.0)
        (set `self.Changable_DelayDuration` 0.0)
        (set `self.needoffset` false)
        (set `self.Last Index` 0)))
    (:`then_1`
      (if (`self.linearV`)
        (set `self.Changeable_Radius` 50.0)
        (set `self.Changeable_VacumDistance` 450.0)
        (set `self.Changeable_vac_force` 350.0)
        (set `self.Changeable_speedup` 100.0)
        (set `self.Changeable_vac_forceHigh` 200.0)
        (set `self.Changeable_noiseVacuum` 0.4)
        (set `self.Changable_DelayDuration` 0.4)
        (set `self.needoffset` false)))
    (:`then_2`
      (if (`self.ShortGunV`)
        (`self.BaseGun`)))
    (:`then_3`
      (if (`self.NoiseGunV`)
        (set `self.Changeable_Radius` 45.0)
        (set `self.Changeable_VacumDistance` 550.0)
        (set `self.Changeable_vac_force` 1.0)
        (set `self.Changeable_speedup` -6.0)
        (set `self.Changeable_vac_forceHigh` 1.0)
        (set `self.Changeable_noiseVacuum` 0.4)
        (set `self.Changable_DelayDuration` 0.0)
        (set `self.needoffset` false)
        (set `self.Last Index` 0)))))

(event `reload`
  (`self.end clean`)
  (`KismetSystemLibrary.PrintString` "reloading")
  (`KismetSystemLibrary.RetriggerableDelay` (`self.Chandable time reload`))
  (for _ (range 1 (+ (`self.total_arm`) 1))
    (`self.add arm`)
    (if (== (`self.current_arm`) (`self.total_arm`))
      (break))))

(event `Fire`
  (if (== (`self.Constant`) 1.0)
    (set `self.Constant` -1.0)))

(event `basegun1`
  (`self.BaseGun`))

(event `Sniper2_act`
  (`self.Sniper2`))

(event `isclean`
  (if (== (`self.Constant`) -1.0)
    (set `self.Constant` 1.0)
    (`KismetSystemLibrary.PrintString` "isclean")))

(event `Sniper3_act`
  (`self.Sniper3`)
  (if (`self.Au2`)
    (`self.notnoisebutbad`)
    (`KismetSystemLibrary.PrintString` "polluted")))

(event `Auto2_act`
  (`self.Auto2`))

(event `Auto3_act`
  (`self.Auto3`)
  (if (`self.Sn2`)
    (`self.noise`)
    (`KismetSystemLibrary.PrintString` "pollutedNoise")))

(fn `add arm`
  (bind _output_get (set `self.current_arm` (- (`self.current_arm`) -1.0)))
  (`KismetSystemLibrary.PrintString` (`KismetStringLibrary.Conv_DoubleToString` _output_get)))

(fn `Auto2`
  (set `self.Au2` true)
  (set `self.Changeable_noiseVacuum` (- (`self.Changeable_noiseVacuum`) 1.0))
  (set `self.Changeable_VacumDistance` (+ (`self.Changeable_VacumDistance`) 100.0))
  (set `self.Changeable_Radius` (- (`self.Changeable_Radius`) 15.0))
  (set `self.Chandable time reload` (+ (`self.Chandable time reload`) -0.3))
  (bind _output_get (set `self.total_arm` (+ (`self.total_arm`) 30)))
  (set `self.current_arm` (`KismetMathLibrary.Conv_IntToDouble` _output_get))
  (set `self.Changeable_vac_force` (+ (`self.Changeable_vac_force`) 30.0)))

(fn `Auto3`
  (set `self.Au3` true)
  (set `self.Changeable_noiseVacuum` (- (`self.Changeable_noiseVacuum`) 0.83))
  (set `self.Changeable_VacumDistance` (+ (`self.Changeable_VacumDistance`) 150.0))
  (set `self.Changeable_Radius` (- (`self.Changeable_Radius`) 10.0))
  (set `self.Chandable time reload` (+ (`self.Chandable time reload`) -0.2))
  (bind _output_get (set `self.total_arm` (+ (`self.total_arm`) 45)))
  (set `self.current_arm` (`KismetMathLibrary.Conv_IntToDouble` _output_get))
  (set `self.Changeable_vac_force` (+ (`self.Changeable_vac_force`) 65.0))
  (set `self.Changeable_vac_forceHigh` (+ (`self.Changeable_vac_forceHigh`) 155.0))
  (set `self.Changeable_speedup` 100.0)
  (set `self.Changable_DelayDuration` 0.0)
  (set `self.needoffset` true)
  (set `self.Last Index` 0))

(fn `BaseGun`
  (set `self.Changeable_Radius` 95.0)
  (set `self.Changeable_VacumDistance` 100.0)
  (set `self.Changeable_vac_force` 100.0)
  (set `self.Changeable_speedup` 50.0)
  (set `self.Changeable_vac_forceHigh` 100.0)
  (set `self.Changeable_noiseVacuum` 2.0)
  (set `self.Changable_DelayDuration` 0.0)
  (set `self.needoffset` true)
  (set `self.Last Index` 0)
  (set `self.current_arm` 45.0)
  (set `self.total_arm` 45)
  (set `self.Chandable time reload` 1.0))

(fn `change arm`
  (bind _output_get (set `self.current_arm` (- (`self.current_arm`) 1.0)))
  (`KismetSystemLibrary.PrintString` (`KismetStringLibrary.Conv_DoubleToString` _output_get)))

(fn `find_distance`
  (set `self.distance` (- (`self.vacuumsocket`) (* (`SceneComponent.K2_GetComponentLocation` (`self.fishbase`)) (`self.Constant`)))))

(fn `find_offset`
  (if (`self.needoffset`)
    (set `self.offset` (* (`KismetMathLibrary.Normal` (`SceneComponent.GetForwardVector` (`self.Follow Camera`))) 100.0))))

(fn `noise`
  (set `self.Changeable_noiseVacuum` (+ (`self.Changeable_noiseVacuum`) 1.5)))

(fn `notnoisebutbad`
  (set `self.total_arm` 50)
  (set `self.current_arm` 50.0))

(fn `Sniper2`
  (set `self.Sn2` true)
  (set `self.Changeable_noiseVacuum` (- (`self.Changeable_noiseVacuum`) 1.2))
  (set `self.Changeable_VacumDistance` (+ (`self.Changeable_VacumDistance`) 150.0))
  (set `self.Changeable_Radius` (- (`self.Changeable_Radius`) 38.0))
  (set `self.Chandable time reload` (+ (`self.Chandable time reload`) 0.5))
  (bind _output_get (set `self.total_arm` (+ (`self.total_arm`) 40)))
  (set `self.current_arm` (`KismetMathLibrary.Conv_IntToDouble` _output_get))
  (set `self.Changeable_vac_force` (+ (`self.Changeable_vac_force`) 75.0))
  (set `self.Changeable_vac_forceHigh` (+ (`self.Changeable_vac_forceHigh`) 75.0))
  (set `self.Changeable_speedup` 100.0)
  (set `self.Changable_DelayDuration` 0.0)
  (set `self.needoffset` true)
  (set `self.Last Index` 0))

(fn `Sniper3`
  (set `self.Sn3` true)
  (set `self.Changeable_noiseVacuum` (- (`self.Changeable_noiseVacuum`) 0.73))
  (set `self.Changeable_VacumDistance` (+ (`self.Changeable_VacumDistance`) 400.0))
  (set `self.Changeable_Radius` (- (`self.Changeable_Radius`) 32.0))
  (set `self.Chandable time reload` (+ (`self.Chandable time reload`) 0.5))
  (bind _output_get (set `self.total_arm` (+ (`self.total_arm`) 0)))
  (set `self.current_arm` (`KismetMathLibrary.Conv_IntToDouble` _output_get))
  (set `self.Changeable_vac_force` (+ (`self.Changeable_vac_force`) 155.0))
  (set `self.Changeable_vac_forceHigh` (+ (`self.Changeable_vac_forceHigh`) 155.0))
  (set `self.Changeable_speedup` 100.0)
  (set `self.Changable_DelayDuration` 0.0)
  (set `self.needoffset` true)
  (set `self.Last Index` 0))

(fn `SpawnFish`
  (bind _returnvalue (`|SpawnActorFromClass` "/Game/weaponsystem/WholeVacuumedStuff/BP_FishBase.BP_FishBase_C" (`KismetMathLibrary.MakeTransform` (+ (`SceneComponent.K2_GetComponentLocation` (`self.Scene`)) (`self.offset`) (* (`KismetMathLibrary.Normal` (`self.GetActorForwardVector` (`self.As BP Third Person Character`))) (100.0 100.0 100.0))) (`SceneComponent.K2_GetComponentRotation` (`self.Scene`))) "AdjustIfPossibleButAlwaysSpawn" "MultiplyWithRoot" null null))
  (set `/Game/weaponsystem/WholeVacuumedStuff/BP_FishBase.impatron` true _returnvalue)
  (`KismetSystemLibrary.PrintString` (`KismetSystemLibrary.GetDisplayName` _returnvalue))
  (`PrimitiveComponent.SetAllPhysicsLinearVelocity` (`/Game/weaponsystem/WholeVacuumedStuff/BP_FishBase.er` _returnvalue) (* (`KismetMathLibrary.Normal` (`SceneComponent.GetForwardVector` (`/Game/ThirdPerson/Blueprints/BP_ThirdPersonCharacter.FollowCamera` (`self.As BP Third Person Character`)))) 10000.0) true))

(fn `UserConstructionScript`)