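; BP_CraftCircle is a moving craft-table target that briefly captures a fish before flinging it away.
; A timeline shifts it along Y from BeginPlay and stops when a BP_FishBase overlaps while none is held.
; After a retriggerable delay, it resumes moving, clears the fish's Blh flag, resets damping and launches it in a random direction.
; The fish reference clears after a second short delay, preventing immediate re-capture; ending overlap also restarts movement.
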(event `play`
  (bind (_returnvalue_x _returnvalue_y _returnvalue_z) (`KismetMathLibrary.BreakVector` (`self.K2_GetActorLocation`)))
  ;[0.15 0 0.09607 0.5] стремное движение мишени-крафт стола
  (set `self.loc` (`self.K2_GetActorLocation`) :!label _label)
  (bind (_direction _newtrack_0) (`Timeline|movement` :!label _label_2)
    (:`Update`
      (set `self.New Track 0` _newtrack_0)
      (`self.K2_SetActorLocation` (`KismetMathLibrary.MakeVector` _returnvalue_x (+ (* _newtrack_0 5.0 (`self.const`)) _returnvalue_y) _returnvalue_z)))))

(event `timer`
  (bind _as_bp_fish_base (`self.As BP Fish Base`))
  (bind _er (`/Game/weaponsystem/WholeVacuumedStuff/BP_FishBase.er` _as_bp_fish_base))
  ;[0.15 0 0.08085 0.5] это таймер когда он проходит крафт стол начинает двигаться и рыба улетает в тартарары или чебоксары как решит рандом
  (`KismetSystemLibrary.RetriggerableDelay` 3.0)
  ;; то что в бегин плее
  (`self.play`)
  (`/Engine/EditorBlueprintResources/StandardMacros.IsValid` _as_bp_fish_base
    (:`Is Valid`
      ;; перестает застревать застывать
      (set `/Game/weaponsystem/WholeVacuumedStuff/BP_FishBase.blh` false _as_bp_fish_base)
      (`PrimitiveComponent.SetLinearDamping` _er 1.0)
      (`PrimitiveComponent.SetAngularDamping` _er 4.0)
      (`PrimitiveComponent.SetAllPhysicsLinearVelocity` _er (* (`KismetMathLibrary.RandomUnitVector`) 3000.0) true)
      (`KismetSystemLibrary.PrintString` "IMFREE BROO" true true (struct :`R` 0.179625 :`G` 1.0 :`A` 1.0))
      ;; рыба успевает убежать и не залипнуть назад в стол
      (`KismetSystemLibrary.RetriggerableDelay` 0.6)
      (set `self.As BP Fish Base` null))))

(event `self.ReceiveBeginPlay`
  ;[0.15 0 0.09607 0.5] стремное движение мишени-крафт стола
  (goto _label))

(event `stopp`
  ;[0.15 0 0.09607 0.5] стремное движение мишени-крафт стола
  (goto _label_2 :!via `Stop`))

(event `self.ReceiveActorBeginOverlap`
  (params (OtherActor :type "Actor Object Reference"))
  ;[0.1365 0.7396 0.003852 0.5] обраткоо тут рыба влипает конкретно
  (bind _asbp_fish_base (cast `/Game/weaponsystem/WholeVacuumedStuff/BP_FishBase` OtherActor))
  (`/Engine/EditorBlueprintResources/StandardMacros.IsValid` (`self.As BP Fish Base`)
    (:`Is Not Valid`
      (set `self.As BP Fish Base` _asbp_fish_base)
      (set `self.move` false)
      ;; стопает таймлайн
      (`self.stopp`)
      (`self.timer`))))

(event `self.ReceiveActorEndOverlap`
  (params (OtherActor :type "Actor Object Reference"))
  ;[0.15 0 0.08684 0.5] херомантия начинает двигаться снова
  (cast `/Game/weaponsystem/WholeVacuumedStuff/BP_FishBase` OtherActor)
  (set `self.move` true)
  (`self.play`))

(fn `UserConstructionScript`)