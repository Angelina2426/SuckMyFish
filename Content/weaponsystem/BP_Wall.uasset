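; BP_Wall is a breakable rock wall that counts down hits from fish and then destroys itself.
; Each overlap by a BP_FishBase with its Impatron flag set decrements CurrentCount.
; Once the decremented count minus one is below one, RockToDestroy plays its break animation and the actor is destroyed after a short delay.
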(event `self.ReceiveActorBeginOverlap`
  (params (OtherActor :type "Actor Object Reference"))
  (bind _returnvalue (- (`self.current count`) 1.0))
  (bind _asbp_fish_base (cast `/Game/weaponsystem/WholeVacuumedStuff/BP_FishBase` OtherActor))
  (if (`/Game/weaponsystem/WholeVacuumedStuff/BP_FishBase.impatron` _asbp_fish_base)
    (set `self.current count` _returnvalue)
    (if (< _returnvalue 1.0)
      (`SkeletalMeshComponent.PlayAnimation` (`self.rock_to_destroy`) "/Game/ThirdPerson/foliage/rock_to_destroy_Anim.rock_to_destroy_Anim" false)
      (`KismetSystemLibrary.Delay` 0.7)
      (`self.K2_DestroyActor`))))

(fn `UserConstructionScript`)