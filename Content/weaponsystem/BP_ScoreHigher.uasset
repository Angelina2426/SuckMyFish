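; BP_ScoreHigher is a pickup actor that overwrites the ScoreFish value on the player's vacuum weapon with its own ScoreFish value.
; On BeginPlay it caches the VacCleanWeapon reference from player 0's BP_ThirdPersonCharacter.
; When a BP_ThirdPersonCharacter overlaps it, it casts that cached weapon to BP_Weapon, assigns the value, then destroys itself after a short delay.
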(event `self.ReceiveBeginPlay`
  (bind _asbp_third_person_character (cast `/Game/ThirdPerson/Blueprints/BP_ThirdPersonCharacter` (`GameplayStatics.GetPlayerCharacter` 0)))
  (set `self.Vac Clean Weapon` (`/Game/ThirdPerson/Blueprints/BP_ThirdPersonCharacter.VacCleanWeapon` _asbp_third_person_character)))

(event `self.ReceiveActorBeginOverlap`
  (params (OtherActor :type "Actor Object Reference"))
  (cast `/Game/ThirdPerson/Blueprints/BP_ThirdPersonCharacter` OtherActor)
  (bind _asbp_weapon (cast `/Game/weaponsystem/BP_Weapon` (`self.Vac Clean Weapon`)))
  (set `/Game/weaponsystem/BP_Weapon.ScoreFish` (`self.Score Fish`) _asbp_weapon)
  (`KismetSystemLibrary.Delay` 0.2)
  (`self.K2_DestroyActor`))

(fn `UserConstructionScript`)