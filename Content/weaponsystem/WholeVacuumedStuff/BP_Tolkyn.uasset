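; BP_Tolkyn is a physics-driven fish enemy with a health widget that swims toward the player while they overlap.
; Overlap pauses the swim timer and adds velocity toward the player each tick, resuming 1.5 seconds after exit.
; Tick also smoothly orients the mesh along velocity and, while Vaccumbro is set, runs a line trace meant to speed up nearby fish.
; Fish flagged as ammo (Impatron) damage it on overlap until Death.
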(event `faster fishh`
  (`self.Linetrace(Tolkyn)`))

(event `self.ReceiveBeginPlay`
  (`|ExecutionSequence`
    (:`then_0`
      ;[0.15 0 0.03162 0.5] рыба выбирает будет она доброй или доброй и косой
      (set `self.Fish Behavior` (`KismetMathLibrary.RandomFloatInRange` -1.0 1.0))
      (set `self.playerpawn` (`GameplayStatics.GetPlayerPawn` 0))
      (set `self.Home` (`SceneComponent.K2_GetComponentLocation` (`self.er`)))
      (`self.Tolkyn_Timer`))
    (:`then_1`
      (bind _aswb_enemy_hp (cast `/Game/weaponsystem/widget/WB_EnemyHP` (`WidgetComponent.GetWidget` (`self.Widget`))))
      (set `/Game/weaponsystem/widget/WB_EnemyHP.MyFish` self _aswb_enemy_hp))))

(event `self.ReceiveTick`
  (params (DeltaSeconds :type "Float (single-precision)"))
  (bind _fish (`self.fish`))
  ;[0.15 0.01987 0.0863 0.5] rotation
  (`SceneComponent.K2_SetWorldRotation` _fish (`KismetMathLibrary.RInterpTo` (`SceneComponent.K2_GetComponentRotation` _fish) (`KismetMathLibrary.Quat_Rotator` (`KismetMathLibrary.Conv_VectorToQuaternion` (* (`KismetMathLibrary.Normal` (stale _returnvalue)) -1.0))) DeltaSeconds 5.0) false false)
  (bind _returnvalue (`PrimitiveComponent.GetPhysicsLinearVelocity` (`self.er`) "None"))
  (`|ExecutionSequence`
    (:`then_0`
      (if (`self.player_here2`)
        (`PrimitiveComponent.SetAllPhysicsLinearVelocity` (`self.er`) (* (- (`self.K2_GetActorLocation` (`self.playerpawn`)) (`SceneComponent.K2_GetComponentLocation` (`self.er`))) 0.05) true)))
    (:`then_1`
      ;[0.15 0.0126 0.09069 0.5] ускоряет рыб рядом
      (if (`self.vaccumbro`)
        (`self.faster fishh`)))))

(event `self.ReceiveActorBeginOverlap`
  (params (OtherActor :type "Actor Object Reference"))
  (`|ExecutionSequence`
    (:`then_0`
      (cast `/Game/ThirdPerson/Blueprints/BP_ThirdPersonCharacter` OtherActor)
      (set `self.player_here2` true)
      (`KismetSystemLibrary.K2_PauseTimerHandle` (`self.swim`)))
    (:`then_1`
      (bind _asbp_fish_base (cast `/Game/weaponsystem/WholeVacuumedStuff/BP_FishBase` OtherActor))
      (if (`/Game/weaponsystem/WholeVacuumedStuff/BP_FishBase.impatron` _asbp_fish_base)
        (bind _output_get (set `self.Current HP` (- (`self.Current HP`) 10.0)))
        (set `/Game/weaponsystem/WholeVacuumedStuff/BP_FishBase.impatron` false _asbp_fish_base)
        (`KismetSystemLibrary.PrintString` (`KismetStringLibrary.Conv_DoubleToString` _output_get) true true (struct :`R` 1.0 :`G` 0.004047 :`B` 0.174456 :`A` 1.0))
        (if (< _output_get 1.0)
          (`self.death`))))))

(event `self.ReceiveActorEndOverlap`
  (params (OtherActor :type "Actor Object Reference"))
  (cast `/Game/ThirdPerson/Blueprints/BP_ThirdPersonCharacter` OtherActor)
  (`KismetSystemLibrary.RetriggerableDelay` 1.5)
  (set `self.player_here2` false)
  (`KismetSystemLibrary.K2_UnPauseTimerHandle` (`self.swim`)))

(fn `UserConstructionScript`
  (`parent.UserConstructionScript`))