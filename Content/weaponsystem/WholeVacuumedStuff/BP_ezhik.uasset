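; BP_ezhik is a vacuumable-stuff creature with an HP widget, which loses health when overlapped by a BP_FishBase flagged as ammo (Impatron).
; Each hit clears that flag and subtracts HP, calling Death below one.
; Tick turns the Fish component opposite to its physics velocity and faces the widget toward the camera.
; An escape event, commented as fleeing after attacking a rat, adds velocity along the normalized world position, away from world origin.
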(event `self.ReceiveBeginPlay`
  (`|ExecutionSequence`
    (:`then_0`
      (`parent.ReceiveBeginPlay`))
    (:`then_1`
      (bind _aswb_enemy_hp (cast `/Game/weaponsystem/widget/WB_EnemyHP` (`WidgetComponent.GetWidget` (`self.Widget`))))
      (set `/Game/weaponsystem/widget/WB_EnemyHP.MyFish` self _aswb_enemy_hp))))

(event `self.ReceiveActorBeginOverlap`
  (params (OtherActor :type "Actor Object Reference"))
  (`parent.ReceiveActorBeginOverlap` OtherActor)
  (bind _asbp_fish_base (cast `/Game/weaponsystem/WholeVacuumedStuff/BP_FishBase` OtherActor))
  (if (`/Game/weaponsystem/WholeVacuumedStuff/BP_FishBase.impatron` _asbp_fish_base)
    (bind _output_get (set `self.Current HP` (- (`self.Current HP`) 25.0)))
    (set `/Game/weaponsystem/WholeVacuumedStuff/BP_FishBase.impatron` false _asbp_fish_base)
    (`KismetSystemLibrary.PrintString` (`KismetStringLibrary.Conv_DoubleToString` _output_get) true true (struct :`R` 1.0 :`G` 0.004047 :`B` 0.174456 :`A` 1.0))
    (if (< _output_get 1.0)
      (`self.death`))))

(event `i need esc`
  ;[0 0.15 0.002095 0.5] убегание после атаки в крысу
  (`PrimitiveComponent.SetAllPhysicsLinearVelocity` (`self.er`) (* (`KismetMathLibrary.Normal` (`SceneComponent.K2_GetComponentLocation` (`self.er`))) 170.0) true))

(event `self.ReceiveTick`
  (params (DeltaSeconds :type "Float (single-precision)"))
  (bind _widget (`self.Widget`))
  (bind _fish (`self.fish`))
  ; rotation
  (bind _returnvalue (`PrimitiveComponent.GetPhysicsLinearVelocity` (`self.er`) "None"))
  (`SceneComponent.K2_SetWorldRotation` _fish (`KismetMathLibrary.RInterpTo` (`SceneComponent.K2_GetComponentRotation` _fish) (`KismetMathLibrary.Quat_Rotator` (`KismetMathLibrary.Conv_VectorToQuaternion` (* (`KismetMathLibrary.Normal` _returnvalue) -1.0))) DeltaSeconds 5.0) false false)
  (`SceneComponent.K2_SetWorldRotation` (`self.Widget`) (`KismetMathLibrary.FindLookAtRotation` (`self.K2_GetActorLocation`) (`self.K2_GetActorLocation` (`GameplayStatics.GetPlayerPawn` 0))) false false)
  (`SceneComponent.K2_SetWorldRotation` _widget (`KismetMathLibrary.FindLookAtRotation` (`SceneComponent.K2_GetComponentLocation` _widget) (`PlayerCameraManager.GetCameraLocation` (`GameplayStatics.GetPlayerCameraManager` 0))) false false))

(fn `UserConstructionScript`
  (`parent.UserConstructionScript`))