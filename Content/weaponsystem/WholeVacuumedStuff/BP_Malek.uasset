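; BP_Malek is an actor in the weapon system's vacuumed-stuff folder with a fish component that turns to follow its physics motion.
; On BeginPlay it applies a material to the Musya component.
; Each Tick it reads the linear velocity of the Er component and smoothly interpolates Fish's world rotation toward one derived from the reversed, normalized velocity.
; The overlap event and construction script add no logic of their own.
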(event `self.ReceiveBeginPlay`
  (`parent.ReceiveBeginPlay`)
  (`PrimitiveComponent.SetMaterial` (`self.Musya`) 0 (`self.Material`)))

(event `self.ReceiveActorBeginOverlap`
  (params (OtherActor :type "Actor Object Reference")))

(event `self.ReceiveTick`
  (params (DeltaSeconds :type "Float (single-precision)"))
  (bind _fish (`self.fish`))
  ; rotation
  (bind _returnvalue (`PrimitiveComponent.GetPhysicsLinearVelocity` (`self.er`) "None"))
  (`SceneComponent.K2_SetWorldRotation` _fish (`KismetMathLibrary.RInterpTo` (`SceneComponent.K2_GetComponentRotation` _fish) (`KismetMathLibrary.Quat_Rotator` (`KismetMathLibrary.Conv_VectorToQuaternion` (* (`KismetMathLibrary.Normal` _returnvalue) -1.0))) DeltaSeconds 5.0) false false))

(fn `UserConstructionScript`
  (`parent.UserConstructionScript`))