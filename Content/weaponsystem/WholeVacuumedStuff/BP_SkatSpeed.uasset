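; A stingray ("skat") actor that gives an overlapping third-person character a boost while it is angry.
; Depending on the speedy flag it calls the character's Speedup or launches them upward, then clears its angry state (delayed after a launch) and calls Mat1.
; Each tick the fish mesh smoothly rotates opposite its physics body's normalized velocity.
; The random behavior setup and Skat call are disconnected.
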(event `self.ReceiveActorBeginOverlap`
  (params (OtherActor :type "Actor Object Reference"))
  ;[0.15 0 0.07859 0.5] прыг скок буст
  (if (`self.angryskat`)
    (`KismetSystemLibrary.PrintString` "JUMP" true true (struct :`R` 1.0 :`G` 0.948746 :`A` 1.0))
    (bind _asbp_third_person_character (cast `/Game/ThirdPerson/Blueprints/BP_ThirdPersonCharacter` OtherActor))
    (if (`self.ifspeedyskat`)
      (`/Game/ThirdPerson/Blueprints/BP_ThirdPersonCharacter.speedup` _asbp_third_person_character)
      (set `self.angryskat` false)
      (else
        (`Character.LaunchCharacter` _asbp_third_person_character (0.0 0.0 1200.0) false true)
        (`KismetSystemLibrary.Delay` 1.0)
        (set `self.angryskat` false)))
    (`self.mat1`)))

(event `self.ReceiveBeginPlay`
  ;[0.15 0.03208 0.05457 0.5] ехал пепе через шнайне видит пепе ватафа
)

(event `self.ReceiveTick`
  (params (DeltaSeconds :type "Float (single-precision)"))
  (bind _fish (`self.fish`))
  ;[0.15 0 0.07073 0.5] rotation to movement
  (bind _returnvalue (`PrimitiveComponent.GetPhysicsLinearVelocity` (`self.er`) "None"))
  (`SceneComponent.K2_SetWorldRotation` _fish (`KismetMathLibrary.RInterpTo` (`SceneComponent.K2_GetComponentRotation` _fish) (`KismetMathLibrary.Quat_Rotator` (`KismetMathLibrary.Conv_VectorToQuaternion` (* (`KismetMathLibrary.Normal` _returnvalue) -1.0))) DeltaSeconds 5.0) false false))

(fn `UserConstructionScript`
  (`parent.UserConstructionScript`))