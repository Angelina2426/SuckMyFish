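; BP_CoralSpot is a trigger actor that spawns a coral when a flagged fish actor overlaps it.
; An overlapping BP_FishBase with Impatron set spawns a BP_Coral_Child while Attempt is above zero, then zeroes Attempt.
; The spawn point combines the spot's XY, shifted opposite the player's forward vector, with a height above the player.
; The new coral gets its Coral flag and an upward physics velocity.
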(event `self.ReceiveActorBeginOverlap`
  (params (OtherActor :type "Actor Object Reference"))
  (bind (_returnvalue_x _returnvalue_y) (`KismetMathLibrary.BreakVector` (`self.K2_GetActorLocation`)))
  (bind _returnvalue (`GameplayStatics.GetPlayerPawn` 0))
  ;[0.09749 0.8698 0 0.5] это корал спот который спавнит коралы тут бы навалить обратки
  (if (> (`self.attempt`) 0)
    (bind _asbp_fish_base (cast `/Game/weaponsystem/WholeVacuumedStuff/BP_FishBase` OtherActor))
    (if (`/Game/weaponsystem/WholeVacuumedStuff/BP_FishBase.impatron` _asbp_fish_base)
      (bind _returnvalue_2 (`|SpawnActorFromClass` "/Game/weaponsystem/WholeVacuumedStuff/BP_Coral_Child.BP_Coral_Child_C" (`KismetMathLibrary.Conv_VectorToTransform` (+ (`KismetMathLibrary.MakeVector` _returnvalue_x _returnvalue_y (+ (.z (`self.K2_GetActorLocation` _returnvalue)) 150.0)) (`KismetMathLibrary.MakeVector` (* (.x (`self.GetActorForwardVector` _returnvalue)) -500.0) (* (.y (`self.GetActorForwardVector` _returnvalue)) -500.0) (.z (`self.GetActorForwardVector` _returnvalue))))) "Undefined" "MultiplyWithRoot" null null))
      (set `/Game/weaponsystem/WholeVacuumedStuff/BP_FishBase.coral` true _returnvalue_2)
      (`PrimitiveComponent.SetAllPhysicsLinearVelocity` (`/Game/weaponsystem/WholeVacuumedStuff/BP_FishBase.er` _returnvalue_2) (0.0 0.0 200.0) false)
      (set `self.attempt` 0))))

(fn `UserConstructionScript`)