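; BP_CraftCircle is a craft-table target actor meant to move along Y on a timeline and catch BP_FishBase fish.
; An overlapping fish is stored if none is held, and the timeline is stopped.
; The Play and Timer events are empty: timeline start and delayed random-velocity fish release are disconnected, so neither runs.
; Tick rotates the widget to face the player camera.
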(event `play`
  ;[0.15 0 0.09607 0.5] стремное движение мишени-крафт стола
)

(event `timer`
  ;[0.15 0 0.08085 0.5] это таймер когда он проходит крафт стол начинает двигаться и рыба улетает в тартарары или чебоксары как решит рандом
)

(event `self.ReceiveBeginPlay`
  ;[0.15 0 0.09607 0.5] стремное движение мишени-крафт стола
)

(event `stopp`
  (bind (_returnvalue_x _returnvalue_y _returnvalue_z) (`KismetMathLibrary.BreakVector` (`self.K2_GetActorLocation`)))
  ;[0.15 0 0.09607 0.5] стремное движение мишени-крафт стола
  (bind (_direction _newtrack_0) (`Timeline|movement` :!via `Stop`)
    (:`Update`
      (set `self.New Track 0` _newtrack_0)
      (`self.K2_SetActorLocation` (`KismetMathLibrary.MakeVector` _returnvalue_x (+ (* _newtrack_0 5.0 (`self.const`)) _returnvalue_y) _returnvalue_z)))))

(event `self.ReceiveActorBeginOverlap`
  (params (OtherActor :type "Actor Object Reference"))
  ;[0.1365 0.7396 0.003852 0.5] обраткоо тут рыба влипает конкретно
  (bind _asbp_fish_base (cast `/Game/weaponsystem/WholeVacuumedStuff/BP_FishBase` OtherActor))
  (`/Engine/EditorBlueprintResources/StandardMacros.IsValid` (`self.As BP Fish Base`)
    (:`Is Not Valid`
      (set `self.As BP Fish Base` _asbp_fish_base)
      (set `self.move` false)
      ;; стопает таймлайн
      (`self.stopp`)
      (`self.timer`))))

(event `self.ReceiveActorEndOverlap`
  (params (OtherActor :type "Actor Object Reference"))
  ;[0.15 0 0.08684 0.5] херомантия начинает двигаться снова
  (cast `/Game/weaponsystem/WholeVacuumedStuff/BP_FishBase` OtherActor)
  (set `self.move` true)
  (`self.play`))

(event `self.ReceiveTick`
  (params (DeltaSeconds :type "Float (single-precision)"))
  (bind _widget (`self.Widget`))
  (`SceneComponent.K2_SetWorldRotation` _widget (`KismetMathLibrary.FindLookAtRotation` (`SceneComponent.K2_GetComponentLocation` _widget) (`PlayerCameraManager.GetCameraLocation` (`GameplayStatics.GetPlayerCameraManager` 0))) false false))

(fn `UserConstructionScript`)